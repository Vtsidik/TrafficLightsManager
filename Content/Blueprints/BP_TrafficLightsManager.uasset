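; Traffic light manager Blueprint that endlessly cycles three referenced lights through red, yellow and green phases.
; The construction script assigns Red, Yellow and Green from the TrafficLights array.
; From BeginPlay, a delay-driven loop via the Recolor event flips IsReverseTrafficLight to alternate red-yellow and green-yellow sequences.
; Each Turn function calls ChangeColor on all three lights, using colors looked up by enum in the ColorSettings map.
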(event `self.ReceiveBeginPlay`
  (if (not (`self.IsReverseTrafficLight?`)) :!label _label
    (`self.TurnRed`)
    (`KismetSystemLibrary.Delay` (`self.RtoY`))
    (`self.TurnYellow`)
    (`KismetSystemLibrary.Delay` (`self.YtoG`))
    (set `self.IsReverseTrafficLight?` true)
    (else
      (`self.TurnGreen`)
      (`KismetSystemLibrary.Delay` (`self.GtoY`))
      (`self.TurnYellow`)
      (`KismetSystemLibrary.Delay` (`self.YtoR`))
      (set `self.IsReverseTrafficLight?` false)))
  (`self.Recolor`))

(event `Recolor`
  (goto _label))

(fn `TurnGreen`
  (bind _colorsettings_colormap (break `/Game/Blueprints/S_LIghtColor` (`self.ColorSettings`)))
  (bind _colorsettings_colormap_2 (break `/Game/Blueprints/S_LIghtColor` (`self.ColorSettings`)))
  (bind _colorsettings_colormap_3 (break `/Game/Blueprints/S_LIghtColor` (`self.ColorSettings`)))
  (bind _output_get (set `self.CurrentColor` "NewEnumerator3"))
  (bind _red (`self.Red`)
    (:`then`
      (`/Game/Blueprints/BP_TraffictLight.ChangeColor` _red (`BlueprintMapLibrary.Map_Find` _colorsettings_colormap _output_get))
      (bind _output_get_2 (set `self.CurrentColor` "NewEnumerator3"))
      (bind _yellow (`self.Yellow`)
        (:`then`
          (`/Game/Blueprints/BP_TraffictLight.ChangeColor` _yellow (`BlueprintMapLibrary.Map_Find` _colorsettings_colormap_3 _output_get_2))
          (bind _output_get_3 (set `self.CurrentColor` "NewEnumerator2"))
          (bind _green (`self.Green`)
            (:`then`
              (`/Game/Blueprints/BP_TraffictLight.ChangeColor` _green (`BlueprintMapLibrary.Map_Find` _colorsettings_colormap_2 _output_get_3)))
            (:`else`)))
        (:`else`)))
    (:`else`)))

(fn `TurnRed`
  (bind _colorsettings_colormap (break `/Game/Blueprints/S_LIghtColor` (`self.ColorSettings`)))
  (bind _colorsettings_colormap_2 (break `/Game/Blueprints/S_LIghtColor` (`self.ColorSettings`)))
  (bind _colorsettings_colormap_3 (break `/Game/Blueprints/S_LIghtColor` (`self.ColorSettings`)))
  (bind _output_get (set `self.CurrentColor` "NewEnumerator0"))
  (bind _red (`self.Red`)
    (:`then`
      (`/Game/Blueprints/BP_TraffictLight.ChangeColor` _red (`BlueprintMapLibrary.Map_Find` _colorsettings_colormap _output_get))
      (bind _output_get_2 (set `self.CurrentColor` "NewEnumerator3"))
      (bind _yellow (`self.Yellow`)
        (:`then`
          (`/Game/Blueprints/BP_TraffictLight.ChangeColor` _yellow (`BlueprintMapLibrary.Map_Find` _colorsettings_colormap_3 _output_get_2))
          (bind _output_get_3 (set `self.CurrentColor` "NewEnumerator3"))
          (bind _green (`self.Green`)
            (:`then`
              (`/Game/Blueprints/BP_TraffictLight.ChangeColor` _green (`BlueprintMapLibrary.Map_Find` _colorsettings_colormap_2 _output_get_3)))
            (:`else`)))
        (:`else`)))
    (:`else`)))

(fn `TurnYellow`
  (bind _colorsettings_colormap (break `/Game/Blueprints/S_LIghtColor` (`self.ColorSettings`)))
  (bind _colorsettings_colormap_2 (break `/Game/Blueprints/S_LIghtColor` (`self.ColorSettings`)))
  (bind _colorsettings_colormap_3 (break `/Game/Blueprints/S_LIghtColor` (`self.ColorSettings`)))
  (bind _output_get (set `self.CurrentColor` "NewEnumerator3"))
  (bind _red (`self.Red`)
    (:`then`
      (`/Game/Blueprints/BP_TraffictLight.ChangeColor` _red (`BlueprintMapLibrary.Map_Find` _colorsettings_colormap _output_get))
      (bind _output_get_2 (set `self.CurrentColor` "NewEnumerator1"))
      (bind _yellow (`self.Yellow`)
        (:`then`
          (`/Game/Blueprints/BP_TraffictLight.ChangeColor` _yellow (`BlueprintMapLibrary.Map_Find` _colorsettings_colormap_3 _output_get_2))
          (bind _output_get_3 (set `self.CurrentColor` "NewEnumerator3"))
          (bind _green (`self.Green`)
            (:`then`
              (`/Game/Blueprints/BP_TraffictLight.ChangeColor` _green (`BlueprintMapLibrary.Map_Find` _colorsettings_colormap_2 _output_get_3)))
            (:`else`)))
        (:`else`)))
    (:`else`)))

(fn `UserConstructionScript`
  (set `self.Red` (`|GetArrayItem` (`self.TrafficLights`)))
  (set `self.Yellow` (`|GetArrayItem` (`self.TrafficLights`) 1))
  (set `self.Green` (`|GetArrayItem` (`self.TrafficLights`) 2)))